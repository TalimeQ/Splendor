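; Player state for a Splendor game that opens a token give-up screen when the player holds too many gem tokens.
; Each tick it reads the first local player's state and, on their turn, checks whether the five gem counts total at least nine.
; It creates the widget once behind a flag, passing it itself, the controller and the token stash, and fills its remaining-count text from the total.
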(event EventBeginPlay
  (Variables|Default|SetBool%20Is%20Created false))

(event EventTick
  (params (DeltaSeconds :type Float%20%28single-precision%29))
  (bind _returnvalue (Game|GetPlayerController 0))
  (bind _asbp_splendor_player_state (Utilities|Casting|CastToBP_SplendorPlayerState (Variables|/Script/Engine.Controller|GetPlayerState (Game|GetPlayerController 0))))
  (if (Class|SplendorPlayerState|GetTurnStatus _asbp_splendor_player_state)
    (if (>= (+ (.emeraldTokens (Utilities|Struct|BreakTokenStruct (Class|SplendorPlayerState|GetPlayerTokens _asbp_splendor_player_state))) (.rubyTokens (Utilities|Struct|BreakTokenStruct (Class|SplendorPlayerState|GetPlayerTokens _asbp_splendor_player_state))) (.onyxTokens (Utilities|Struct|BreakTokenStruct (Class|SplendorPlayerState|GetPlayerTokens _asbp_splendor_player_state))) (.sapphireTokens (Utilities|Struct|BreakTokenStruct (Class|SplendorPlayerState|GetPlayerTokens _asbp_splendor_player_state))) (.diamondTokens (Utilities|Struct|BreakTokenStruct (Class|SplendorPlayerState|GetPlayerTokens _asbp_splendor_player_state)))) 9)
      (if (not (Variables|Default|GetBool%20Is%20Created))
        (Variables|Default|SetBool%20Is%20Created true)
        (bind _returnvalue_2 (UserInterface|CreateWidget "/Game/UI/TestUI/TokenGiveUpUi.TokenGiveUpUi_C" _returnvalue))
        (UserInterface|Viewport|AddtoViewport _returnvalue_2 0)
        (Variables|/Game/UI/TestUI/TokenGiveUpUi.TokenGiveUpUi_C|SetPlayerState _returnvalue_2 self)
        (bind _asbp_splendor_player_cont (Utilities|Casting|CastToBP_SplendorPlayerCont _returnvalue))
        (Variables|/Game/UI/TestUI/TokenGiveUpUi.TokenGiveUpUi_C|SetSplendorPlayerContRef _returnvalue_2 _asbp_splendor_player_cont)
        (Variables|/Game/UI/TestUI/TokenGiveUpUi.TokenGiveUpUi_C|SetTokenStash _returnvalue_2 (Variables|Default|GettokenStashRef))
        (Rendering|Components|TextRender|SetText (Variables|/Game/UI/TestUI/TokenGiveUpUi.TokenGiveUpUi_C|GetCardsRemaining _returnvalue_2) (Utilities|Text|ToText(Integer) (- (+ (.emeraldTokens (Utilities|Struct|BreakTokenStruct (Class|SplendorPlayerState|GetPlayerTokens _asbp_splendor_player_state))) (.rubyTokens (Utilities|Struct|BreakTokenStruct (Class|SplendorPlayerState|GetPlayerTokens _asbp_splendor_player_state))) (.onyxTokens (Utilities|Struct|BreakTokenStruct (Class|SplendorPlayerState|GetPlayerTokens _asbp_splendor_player_state))) (.sapphireTokens (Utilities|Struct|BreakTokenStruct (Class|SplendorPlayerState|GetPlayerTokens _asbp_splendor_player_state))) (.diamondTokens (Utilities|Struct|BreakTokenStruct (Class|SplendorPlayerState|GetPlayerTokens _asbp_splendor_player_state)))) 2)))))))

(fn ConstructionScript)