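; CardStack_BP is a card stack actor in a Splendor game that opens reservation UI for the local player.
; On BeginPlay it binds handlers to its stack-request and no-gold events.
; Each handler creates a reserve widget, the normal or insufficient-gold variant, passes it the player controller and stack references, and toggles input.
; It uses player controller 0, and a TODO flags the no-gold path as not yet networked.
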(event Custom|Event%20OnRaycast
  (bind _returnvalue (Game|GetPlayerController 0))
  (bind _returnvalue_2 (UserInterface|CreateWidget "/Game/UI/TestUI/ReserveFromStackNormal.ReserveFromStackNormal_C" _returnvalue))
  (UserInterface|Viewport|AddtoViewport _returnvalue_2 0)
  (bind _assplendor_player_controller (Utilities|Casting|CastToSplendorPlayerController _returnvalue))
  (Variables|/Game/UI/TestUI/ReserveFromStackNormal.ReserveFromStackNormal_C|SetPlayerContRef _returnvalue_2 _assplendor_player_controller)
  (Class|SplendorPlayerController|ToggleInput _assplendor_player_controller)
  (Variables|/Game/UI/TestUI/ReserveFromStackNormal.ReserveFromStackNormal_C|SetCardStackRef _returnvalue_2 self))

(event Custom|InsufficientGold
  (bind _returnvalue (Game|GetPlayerController 0))
  (bind _returnvalue_2 (UserInterface|CreateWidget "/Game/UI/TestUI/CardReserveStack.CardReserveStack_C" _returnvalue))
  (UserInterface|Viewport|AddtoViewport _returnvalue_2 0)
  (bind _assplendor_player_controller (Utilities|Casting|CastToSplendorPlayerController _returnvalue))
  (bind _output_get (Variables|/Game/UI/TestUI/CardReserveStack.CardReserveStack_C|SetPlayerContRef _returnvalue_2 _assplendor_player_controller))
  (Class|SplendorPlayerController|ToggleInput _output_get)
  (Variables|/Game/UI/TestUI/CardReserveStack.CardReserveStack_C|SetCardStackRef _returnvalue_2 self))

(event EventBeginPlay
  (EventDispatchers|BindEventtoOnCardStackRequest (delegate Custom|Event%20OnRaycast))
  (EventDispatchers|BindEventtoNoGoldMessage (delegate Custom|InsufficientGold)))

(event Collision|EventActorBeginOverlap
  (params (OtherActor :type Actor%20Object%20Reference)))

(event EventTick
  (params (DeltaSeconds :type Float%20%28single-precision%29)))

(fn ConstructionScript)