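; Base game mode for a Splendor card game that sets up shared card visuals and triggers game state initialization.
; BeginPlay spawns four CardVis actors in an evenly spaced line, rotates and half-scales them, stores them in CardRefs, and makes them replicated and always relevant.
; Each PostLogin calls Initialize on SplendorGameState_BP and prints a debug message.
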(event EventTick
  (params (DeltaSeconds :type Float%20%28single-precision%29)))

(event EventPostLogin
  (params (NewPlayer :type Player%20Controller%20Object%20Reference))
  (bind _assplendor_game_state_bp (Utilities|Casting|CastToSplendorGameState_BP (Game|GetGameState)))
  (Class|SplendorGameState|Initialize _assplendor_game_state_bp)
  (Development|PrintString "POST LOGIN"))

(event EventBeginPlay
  (for _index (range 0 3)
    (bind _returnvalue (Game|SpawnActorfromClass "/Game/CardVis.CardVis_C" (Math|Conversions|ToTransform(Vector) (Math|Vector|MakeVector 4.8e+02 (Math|Conversions|ToFloat(Integer) (+ -340 (* 170 _index))) 3e+01)) "AlwaysSpawn" 0 0))
    (Transformation|SetActorRotation _returnvalue "0.000000,90.000000, 0")
    (Transformation|SetActorScale3D _returnvalue "0.500000,0.500000,0.500000")
    (Utilities|Array|Add (Variables|Default|GetCardRefs) _returnvalue)
    (Networking|SetReplicates _returnvalue true)
    (Variables|/Script/Engine.Actor|SetbAlwaysRelevant _returnvalue true)))

(fn ConstructionScript)